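; BP_TestActor is a sandbox actor demonstrating Blueprint and C++ interop, with no active gameplay logic.
; It exposes empty native and implementable event overrides alongside stub Blueprint functions in regular, pure and compact forms.
; Unconnected example nodes show variable access, C++ callable and pure function calls, and random-number prints illustrating pure node evaluation.
; All events are empty, so none of these examples run.
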(event EventBeginPlay)

(event Collision|EventActorBeginOverlap
  (params (OtherActor :type Actor%20Object%20Reference)))

(event EventTick
  (params (DeltaSeconds :type Float%20%28single-precision%29)))

(event EventBlueprintNativeEventFunction
  ;[0.5 0 0.5] CPP функции
  ;;[0 0 0] Часть логики в С++, продолжение в блюпринте
)

(event EventBlueprintImplementableEventFunction
  ;[0.5 0 0.5] CPP функции
  ;;[0 0 0] Вызываем в С++ логику из блюпринта
)

(fn ConstructionScript)

(fn BlueprintFunc)

(fn PureBlueprintFunc
  (return false 0.0))

(fn CompactBlueprintFunc)

(fn PureCompactBlueprintFunc
  (return false 0))