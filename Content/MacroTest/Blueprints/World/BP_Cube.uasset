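; BP_Cube is a test world actor that lights up while the player stands in its trigger area.
; Box component overlap events check that the other actor is player character 0, then show or hide the PointLight.
; Separate actor-level begin and end overlap events print debug messages for any overlapping actor, illustrating actor versus component overlap handling.
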(event OnComponentBeginOverlap(Box)
  (params (OverlappedComponent :type Primitive%20Component%20Object%20Reference) (OtherActor :type Actor%20Object%20Reference) (OtherComp :type Primitive%20Component%20Object%20Reference) (OtherBodyIndex :type Integer) (bFromSweep :type Boolean) (SweepResult :type Hit%20Result%20Structure%20%28by%20ref%29))
  ;[0.5 0 0.5] События пересечения компонента
  (if (== OtherActor (Game|GetPlayerCharacter 0))
    (Rendering|SetVisibility (Variables|Default|GetPointLight) true false)))

(event OnComponentEndOverlap(Box)
  (params (OverlappedComponent :type Primitive%20Component%20Object%20Reference) (OtherActor :type Actor%20Object%20Reference) (OtherComp :type Primitive%20Component%20Object%20Reference) (OtherBodyIndex :type Integer))
  ;[0.5 0 0.5] События пересечения компонента
  (if (== OtherActor (Game|GetPlayerCharacter 0))
    (Rendering|SetVisibility (Variables|Default|GetPointLight) false false)))

(event EventBeginPlay)

(event EventTick
  (params (DeltaSeconds :type Float%20%28single-precision%29)))

(event Collision|EventActorBeginOverlap
  (params (OtherActor :type Actor%20Object%20Reference))
  ;[0.5 0 0.5] События пересечения актора
  (Development|PrintString "Hello! I ActorBeginOverlap =)" true true "(R=0.000000,G=0.000000,B=1.000000,A=1.000000)"))

(event Collision|EventActorEndOverlap
  (params (OtherActor :type Actor%20Object%20Reference))
  ;[0.5 0 0.5] События пересечения актора
  (Development|PrintString "Hello! I ActorEndOverlap =)" true true "(R=0.000000,G=0.000000,B=1.000000,A=1.000000)"))

(fn ConstructionScript)